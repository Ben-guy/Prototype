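; Locked door Blueprint that swings open when the first-person character enters its trigger box holding the matching key.
; On overlap it loops the character's Key boolean array and, if the entry at its KeyNumber index is true, plays the Rotation timeline to set the door's relative yaw.
; Leaving the box reverses the timeline after a short delay, with no check on who left or whether they had the key.
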(event OnComponentBeginOverlap(Box)
  (params (OverlappedComponent :type Primitive%20Component%20Object%20Reference) (OtherActor :type Actor%20Object%20Reference) (OtherComp :type Primitive%20Component%20Object%20Reference) (OtherBodyIndex :type Integer) (bFromSweep :type Boolean) (SweepResult :type Hit%20Result%20Structure%20%28by%20ref%29))
  ;[1 1 1] Checks to see if the key is correct
  (bind _asfirst_person_character (Utilities|Casting|CastToFirstPersonCharacter OtherActor))
  (for (_array_element _array_index) (Variables|/Game/FirstPerson/Blueprints/FirstPersonCharacter.FirstPersonCharacter_C|GetKey _asfirst_person_character)
    (if (and _array_element (== _array_index (Variables|Default|GetKeyNumber)))
      ;[1 1 1] Moves door
      (bind _rotation (Timeline|Rotation Play)
        (:Update
          (Transformation|SetRelativeRotation (Variables|Default|GetDoor) (Math|Rotator|MakeRotator 0.0 0.0 _rotation) false false))))))

(event OnComponentEndOverlap(Box)
  (params (OverlappedComponent :type Primitive%20Component%20Object%20Reference) (OtherActor :type Actor%20Object%20Reference) (OtherComp :type Primitive%20Component%20Object%20Reference) (OtherBodyIndex :type Integer))
  (Utilities|FlowControl|Delay 2.0)
  ;[1 1 1] Moves door
  (bind _rotation (Timeline|Rotation Reverse)
    (:Update
      (Transformation|SetRelativeRotation (Variables|Default|GetDoor) (Math|Rotator|MakeRotator 0.0 0.0 _rotation) false false))))

(fn ConstructionScript)