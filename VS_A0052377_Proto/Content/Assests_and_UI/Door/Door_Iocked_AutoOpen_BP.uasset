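; Locked door Blueprint that opens automatically when the first-person player character holds its key.
; Tick, throttled by a Delay, scans the character's Key boolean array for a true entry at the door's KeyNumber.
; A match plays a timeline that drives the door's relative yaw.
; After a further delay from the timeline update, it spawns Door_Blank_BP at the door's transform and destroys itself as an optimization.
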(event EventTick
  (params (DeltaSeconds :type Float%20%28single-precision%29))
  (bind _door (Variables|Default|GetDoor))
  (Utilities|FlowControl|Delay 0.2)
  ;[1 1 1] Checks to see if the key is correct
  (bind _asfirst_person_character (Utilities|Casting|CastToFirstPersonCharacter (Game|GetPlayerCharacter 0)))
  (for (_array_element _array_index) (Variables|/Game/FirstPerson/Blueprints/FirstPersonCharacter.FirstPersonCharacter_C|GetKey _asfirst_person_character)
    (if (and _array_element (== _array_index (Variables|Default|GetKeyNumber)))
      ;[1 1 1] Moves door
      (bind _rotation (Timeline|Time Play)
        (:Update
          (Transformation|SetRelativeRotation (Variables|Default|GetDoor) (Math|Rotator|MakeRotator 0.0 0.0 _rotation) false false)
          ;[1 1 1] Spawns a blank door and destroys locked door to optimise game
          (Utilities|FlowControl|Delay 5.0)
          (Game|SpawnActorfromClass "/Game/Assests_and_UI/Door/Door_Blank_BP.Door_Blank_BP_C" (Math|Transform|MakeTransform (Transformation|GetWorldLocation _door) (Transformation|GetWorldRotation _door) "1,1,1") "Undefined" 0 0)
          (Actor|DestroyActor))))))

(fn ConstructionScript)