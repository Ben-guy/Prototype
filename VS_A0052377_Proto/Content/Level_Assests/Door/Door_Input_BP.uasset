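; Door Blueprint that lets the player swing a door open with the E key while standing in its trigger box.
; Overlapping the box adds a Door_Input prompt widget and enables player input, so E plays the Rotation timeline that drives the door's relative yaw.
; Leaving the box disables input and reverses the timeline after a short delay; the widget is never removed here.
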(event OnComponentBeginOverlap(Box)
  (params (OverlappedComponent :type Primitive%20Component%20Object%20Reference) (OtherActor :type Actor%20Object%20Reference) (OtherComp :type Primitive%20Component%20Object%20Reference) (OtherBodyIndex :type Integer) (bFromSweep :type Boolean) (SweepResult :type Hit%20Result%20Structure%20%28by%20ref%29))
  ;[1 1 1] Creates UI and enables input from player, when overlapped
  (bind _returnvalue (UserInterface|CreateWidget "/Game/Level_Assests/UI/Door_Input.Door_Input_C"))
  (UserInterface|Viewport|AddtoViewport _returnvalue 0)
  (Input|EnableInput (Game|GetPlayerController 0))
  (Utilities|FlowControl|Delay 3.0))

(event OnComponentEndOverlap(Box)
  (params (OverlappedComponent :type Primitive%20Component%20Object%20Reference) (OtherActor :type Actor%20Object%20Reference) (OtherComp :type Primitive%20Component%20Object%20Reference) (OtherBodyIndex :type Integer))
  ;[1 1 1] Disables input when not overlapped
  (Input|DisableInput 0)
  (Utilities|FlowControl|Delay 2.0)
  ;[1 1 1] If input is enabled, allows for door to be opened when E is pressed
  (bind _rotation (Timeline|Rotation Reverse)
    (:Update
      (Transformation|SetRelativeRotation (Variables|Default|GetDoor) (Math|Rotator|MakeRotator 0.0 0.0 _rotation) false false))))

(event Input|KeyboardEvents|E
  (params (Key :type Key%20Structure :default "None"))
  ;[1 1 1] If input is enabled, allows for door to be opened when E is pressed
  (:Pressed
    (bind _rotation (Timeline|Rotation Play)
      (:Update
        (Transformation|SetRelativeRotation (Variables|Default|GetDoor) (Math|Rotator|MakeRotator 0.0 0.0 _rotation) false false)))))

(fn ConstructionScript)